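; End screen score actor that shows score, time and item count on three text render components.
; On BeginPlay, an Update event fills them with hardcoded placeholder strings rather than real game data.
; Construction script logic to size and vertically space the texts by TextSize and TextOffset is disconnected and never runs.
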(event Custom|Update
  (Rendering|Components|TextRender|SetText (Variables|Default|GetTextRender_Score) (Utilities|Text|ToText(String) (Utilities|String|MakeLiteralString "69420")))
  (Rendering|Components|TextRender|SetText (Variables|Default|GetTextRender_Time) (Utilities|Text|ToText(String) (Utilities|String|MakeLiteralString "4:20")))
  (Rendering|Components|TextRender|SetText (Variables|Default|GetTextRender_Items) (Utilities|Text|ToText(String) (Utilities|String|MakeLiteralString "6/9"))))

(event EventBeginPlay
  (CallFunction|Update))

(event Collision|EventActorBeginOverlap
  (params (OtherActor :type Actor%20Object%20Reference)))

(event EventTick
  (params (DeltaSeconds :type Float%20%28single-precision%29)))

(fn ConstructionScript)