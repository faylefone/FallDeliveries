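; End screen actor that displays one food item and shows whether the player has any of it.
; The construction script and BeginPlay both set the Paper2D sprite from the ItemType enum, so placed instances preview their dish in the editor.
; At BeginPlay it reads that item's count from the Item_Variable_Storage game instance and swaps to a greyed material when the count is not above zero.
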(event EventBeginPlay
  (bind _itemtype (Variables|Default|GetItemType))
  (Rendering|Components|Sprite|SetSprite (Variables|Default|GetPaperSprite) (Utilities|Select :Index _itemtype :NewEnumerator0 "/Game/GameJam/Assets/Sprites/Turkey_Item_Sprite.Turkey_Item_Sprite" :NewEnumerator1 "/Game/GameJam/Assets/Sprites/Salad_Item_Sprite.Salad_Item_Sprite" :NewEnumerator2 "/Game/GameJam/Assets/Sprites/Rolls_Sprite.Rolls_Sprite" :NewEnumerator3 "/Game/GameJam/Assets/Sprites/Pie_Item_Sprite.Pie_Item_Sprite" :NewEnumerator4 "/Game/GameJam/Assets/Sprites/Mash_Tatos_Sprite.Mash_Tatos_Sprite" :NewEnumerator5 "/Game/GameJam/Assets/Sprites/Mac_n_Cheese_Sprite.Mac_n_Cheese_Sprite" :NewEnumerator6 "/Game/GameJam/Assets/Sprites/Jello_Sprite.Jello_Sprite" :NewEnumerator7 "/Game/GameJam/Assets/Sprites/Ham_Item_Sprite.Ham_Item_Sprite" :NewEnumerator8 "/Game/GameJam/Assets/Sprites/Green_Beans_Sprite.Green_Beans_Sprite" :NewEnumerator9 "/Game/GameJam/Assets/Sprites/Gravy_Item_Sprite.Gravy_Item_Sprite" :NewEnumerator10 "/Game/GameJam/Assets/Sprites/Cranberry_Sauce_Sprite.Cranberry_Sauce_Sprite" :NewEnumerator11 "/Game/GameJam/Assets/Sprites/Corn_Item_Sprite.Corn_Item_Sprite" :NewEnumerator12 "/Game/GameJam/Assets/Sprites/Cassarole_Sprite.Cassarole_Sprite" :NewEnumerator13 "/Game/GameJam/Assets/Sprites/Cassarole_CLosed_Sprite.Cassarole_CLosed_Sprite" :NewEnumerator14 "/Game/GameJam/Assets/Sprites/Yellow_Dish_Sprite.Yellow_Dish_Sprite"))
  (bind _asitem_variable_storage (Utilities|Casting|CastToItem_Variable_Storage (Game|GetGameInstance)))
  (switch Utilities|FlowControl|Switch|SwitchonItems _itemtype
    (:NewEnumerator0
      (if (not (> (Variables|/Game/GameJam/Blueprints/Items/Item_Variable_Storage.Item_Variable_Storage_C|GetTurkey _asitem_variable_storage) 0))
        (Rendering|Material|SetMaterial (Variables|Default|GetPaperSprite) 0 "/Game/GameJam/Blueprints/Score_BP/GreyedItemMat.GreyedItemMat" :!label _label)))
    (:NewEnumerator1
      (if (not (> (Variables|/Game/GameJam/Blueprints/Items/Item_Variable_Storage.Item_Variable_Storage_C|GetSalad _asitem_variable_storage) 0))
        (goto _label)))
    (:NewEnumerator2
      (if (not (> (Variables|/Game/GameJam/Blueprints/Items/Item_Variable_Storage.Item_Variable_Storage_C|GetRolls _asitem_variable_storage) 0))
        (goto _label)))
    (:NewEnumerator3
      (if (not (> (Variables|/Game/GameJam/Blueprints/Items/Item_Variable_Storage.Item_Variable_Storage_C|GetPie _asitem_variable_storage) 0))
        (goto _label)))
    (:NewEnumerator4
      (if (not (> (Variables|/Game/GameJam/Blueprints/Items/Item_Variable_Storage.Item_Variable_Storage_C|GetMashTatos _asitem_variable_storage) 0))
        (goto _label)))
    (:NewEnumerator5
      (if (not (> (Variables|/Game/GameJam/Blueprints/Items/Item_Variable_Storage.Item_Variable_Storage_C|GetMacnCheese _asitem_variable_storage) 0))
        (goto _label)))
    (:NewEnumerator6
      (if (not (> (Variables|/Game/GameJam/Blueprints/Items/Item_Variable_Storage.Item_Variable_Storage_C|GetJello _asitem_variable_storage) 0))
        (goto _label)))
    (:NewEnumerator7
      (if (not (> (Variables|/Game/GameJam/Blueprints/Items/Item_Variable_Storage.Item_Variable_Storage_C|GetHam _asitem_variable_storage) 0))
        (goto _label)))
    (:NewEnumerator8
      (if (not (> (Variables|/Game/GameJam/Blueprints/Items/Item_Variable_Storage.Item_Variable_Storage_C|GetGreen%20Beans _asitem_variable_storage) 0))
        (goto _label)))
    (:NewEnumerator9
      (if (not (> (Variables|/Game/GameJam/Blueprints/Items/Item_Variable_Storage.Item_Variable_Storage_C|GetGravy _asitem_variable_storage) 0))
        (goto _label)))
    (:NewEnumerator10
      (if (not (> (Variables|/Game/GameJam/Blueprints/Items/Item_Variable_Storage.Item_Variable_Storage_C|GetCranberry _asitem_variable_storage) 0))
        (goto _label)))
    (:NewEnumerator11
      (if (not (> (Variables|/Game/GameJam/Blueprints/Items/Item_Variable_Storage.Item_Variable_Storage_C|GetCorn _asitem_variable_storage) 0))
        (goto _label)))
    (:NewEnumerator12
      (if (not (> (Variables|/Game/GameJam/Blueprints/Items/Item_Variable_Storage.Item_Variable_Storage_C|GetCassarole _asitem_variable_storage) 0))
        (goto _label)))
    (:NewEnumerator13
      (if (not (> (Variables|/Game/GameJam/Blueprints/Items/Item_Variable_Storage.Item_Variable_Storage_C|GetClosed%20Cassarole _asitem_variable_storage) 0))
        (goto _label)))
    (:NewEnumerator14
      (if (not (> (Variables|/Game/GameJam/Blueprints/Items/Item_Variable_Storage.Item_Variable_Storage_C|GetYellow _asitem_variable_storage) 0))
        (goto _label)))))

(event Collision|EventActorBeginOverlap
  (params (OtherActor :type Actor%20Object%20Reference)))

(event EventTick
  (params (DeltaSeconds :type Float%20%28single-precision%29)))

(fn ConstructionScript
  (Rendering|Components|Sprite|SetSprite (Variables|Default|GetPaperSprite) (Utilities|Select :Index (Variables|Default|GetItemType) :NewEnumerator0 "/Game/GameJam/Assets/Sprites/Turkey_Item_Sprite.Turkey_Item_Sprite" :NewEnumerator1 "/Game/GameJam/Assets/Sprites/Salad_Item_Sprite.Salad_Item_Sprite" :NewEnumerator2 "/Game/GameJam/Assets/Sprites/Rolls_Sprite.Rolls_Sprite" :NewEnumerator3 "/Game/GameJam/Assets/Sprites/Pie_Item_Sprite.Pie_Item_Sprite" :NewEnumerator4 "/Game/GameJam/Assets/Sprites/Mash_Tatos_Sprite.Mash_Tatos_Sprite" :NewEnumerator5 "/Game/GameJam/Assets/Sprites/Mac_n_Cheese_Sprite.Mac_n_Cheese_Sprite" :NewEnumerator6 "/Game/GameJam/Assets/Sprites/Jello_Sprite.Jello_Sprite" :NewEnumerator7 "/Game/GameJam/Assets/Sprites/Ham_Item_Sprite.Ham_Item_Sprite" :NewEnumerator8 "/Game/GameJam/Assets/Sprites/Green_Beans_Sprite.Green_Beans_Sprite" :NewEnumerator9 "/Game/GameJam/Assets/Sprites/Gravy_Item_Sprite.Gravy_Item_Sprite" :NewEnumerator10 "/Game/GameJam/Assets/Sprites/Cranberry_Sauce_Sprite.Cranberry_Sauce_Sprite" :NewEnumerator11 "/Game/GameJam/Assets/Sprites/Corn_Item_Sprite.Corn_Item_Sprite" :NewEnumerator12 "/Game/GameJam/Assets/Sprites/Cassarole_Sprite.Cassarole_Sprite" :NewEnumerator13 "/Game/GameJam/Assets/Sprites/Cassarole_CLosed_Sprite.Cassarole_CLosed_Sprite" :NewEnumerator14 "/Game/GameJam/Assets/Sprites/Yellow_Dish_Sprite.Yellow_Dish_Sprite")))