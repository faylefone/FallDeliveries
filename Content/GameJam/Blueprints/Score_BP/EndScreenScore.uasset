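; EndScreenScore is an end-screen actor that shows the player's score, time and item count on text render components.
; On BeginPlay it casts the Game Instance to Item_Variable_Storage and totals the stored food item counts, each multiplied by a fixed point value.
; Only the score is computed; time and item count are hard-coded strings.
; Text size and offset nodes in the Construction Script are unconnected and never run.
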(event Custom|Update
  (Rendering|Components|TextRender|SetText (Variables|Default|GetTextRender_Score) (Utilities|Text|ToText(String) (Utilities|String|MakeLiteralString (Utilities|String|ToString(Integer) (+ (* (Variables|/Game/GameJam/Blueprints/Items/Item_Variable_Storage.Item_Variable_Storage_C|GetTurkey (stale EventBeginPlay _asitem_variable_storage)) 1500) (* (Variables|/Game/GameJam/Blueprints/Items/Item_Variable_Storage.Item_Variable_Storage_C|GetSalad (stale EventBeginPlay _asitem_variable_storage)) 400) (* (Variables|/Game/GameJam/Blueprints/Items/Item_Variable_Storage.Item_Variable_Storage_C|GetRolls (stale EventBeginPlay _asitem_variable_storage)) 1200) (* (Variables|/Game/GameJam/Blueprints/Items/Item_Variable_Storage.Item_Variable_Storage_C|GetPie (stale EventBeginPlay _asitem_variable_storage)) 1300) (* (Variables|/Game/GameJam/Blueprints/Items/Item_Variable_Storage.Item_Variable_Storage_C|GetMashTatos (stale EventBeginPlay _asitem_variable_storage)) 900) (* (Variables|/Game/GameJam/Blueprints/Items/Item_Variable_Storage.Item_Variable_Storage_C|GetMacnCheese (stale EventBeginPlay _asitem_variable_storage)) 700) (* (Variables|/Game/GameJam/Blueprints/Items/Item_Variable_Storage.Item_Variable_Storage_C|GetJello (stale EventBeginPlay _asitem_variable_storage)) 600) (* (Variables|/Game/GameJam/Blueprints/Items/Item_Variable_Storage.Item_Variable_Storage_C|GetHam (stale EventBeginPlay _asitem_variable_storage)) 1400) (* (Variables|/Game/GameJam/Blueprints/Items/Item_Variable_Storage.Item_Variable_Storage_C|GetGreen%20Beans (stale EventBeginPlay _asitem_variable_storage)) 800) (* (Variables|/Game/GameJam/Blueprints/Items/Item_Variable_Storage.Item_Variable_Storage_C|GetGravy (stale EventBeginPlay _asitem_variable_storage)) 1000) (* (Variables|/Game/GameJam/Blueprints/Items/Item_Variable_Storage.Item_Variable_Storage_C|GetCranberry (stale EventBeginPlay _asitem_variable_storage)) 1100) (* (Variables|/Game/GameJam/Blueprints/Items/Item_Variable_Storage.Item_Variable_Storage_C|GetCorn (stale EventBeginPlay _asitem_variable_storage)) 500) (* (Variables|/Game/GameJam/Blueprints/Items/Item_Variable_Storage.Item_Variable_Storage_C|GetCassarole (stale EventBeginPlay _asitem_variable_storage)) 100) (* (Variables|/Game/GameJam/Blueprints/Items/Item_Variable_Storage.Item_Variable_Storage_C|GetClosed%20Cassarole (stale EventBeginPlay _asitem_variable_storage)) 100) (* (Variables|/Game/GameJam/Blueprints/Items/Item_Variable_Storage.Item_Variable_Storage_C|GetYellow (stale EventBeginPlay _asitem_variable_storage)) 100))))))
  (Rendering|Components|TextRender|SetText (Variables|Default|GetTextRender_Time) (Utilities|Text|ToText(String) (Utilities|String|MakeLiteralString "4:20")))
  (Rendering|Components|TextRender|SetText (Variables|Default|GetTextRender_Items) (Utilities|Text|ToText(String) (Utilities|String|MakeLiteralString "6/9"))))

(event EventBeginPlay
  ;[1 1 1] Item Values + Calculating Score
  (bind _asitem_variable_storage (Utilities|Casting|CastToItem_Variable_Storage (Game|GetGameInstance)))
  (CallFunction|Update))

(event Collision|EventActorBeginOverlap
  (params (OtherActor :type Actor%20Object%20Reference)))

(event EventTick
  (params (DeltaSeconds :type Float%20%28single-precision%29)))

(fn ConstructionScript)