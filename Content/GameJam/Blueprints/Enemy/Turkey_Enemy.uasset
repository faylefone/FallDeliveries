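; Turkey enemy that patrols back and forth while the player is inside its activation sphere, knocking them back on contact.
; On BeginPlay it can snap to the surface below with a sphere trace.
; An overlap-controlled gate on Tick drives forward movement, with a downward look-ahead trace turning it around at ledges.
; DamageSphere hits launch the player away along X and upward, with a turkey sound throttled by a resetting DoOnce.
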(event OnComponentBeginOverlap(ActivationSphere)
  (params (OverlappedComponent :type Primitive%20Component%20Object%20Reference) (OtherActor :type Actor%20Object%20Reference) (OtherComp :type Primitive%20Component%20Object%20Reference) (OtherBodyIndex :type Integer) (bFromSweep :type Boolean) (SweepResult :type Hit%20Result%20Structure%20%28by%20ref%29))
  (bind _returnvalue (Transformation|GetActorTransform))
  (bind _returnvalue_2 (Math|Transform|TransformLocation _returnvalue "100.000000, 0, 0"))
  (if (== (Utilities|GetClass OtherActor) "/Game/GameJam/Blueprints/Player/Player.Player_C")
    (Utilities|FlowControl|Gate true) ; enters at Open
  ))

(event OnComponentEndOverlap(ActivationSphere)
  (params (OverlappedComponent :type Primitive%20Component%20Object%20Reference) (OtherActor :type Actor%20Object%20Reference) (OtherComp :type Primitive%20Component%20Object%20Reference) (OtherBodyIndex :type Integer))
  (bind _returnvalue (Transformation|GetActorTransform))
  (bind _returnvalue_2 (Math|Transform|TransformLocation _returnvalue "100.000000, 0, 0"))
  (if (== (Utilities|GetClass OtherActor) "/Game/GameJam/Blueprints/Player/Player.Player_C")
    (Utilities|FlowControl|Gate true) ; enters at Close
  ))

(event OnComponentHit(DamageSphere)
  (params (HitComponent :type Primitive%20Component%20Object%20Reference) (OtherActor :type Actor%20Object%20Reference) (OtherComp :type Primitive%20Component%20Object%20Reference) (NormalImpulse :type Vector :default "0, 0, 0") (Hit :type Hit%20Result%20Structure%20%28by%20ref%29))
  (bind _knockbackforce (Variables|Default|GetKnockbackForce))
  (bind _asplayer (Utilities|Casting|CastToPlayer OtherActor))
  (Character|LaunchCharacter _asplayer (select (>= (.x (Math|Vector|GetUnitDirection(Vector) (Transformation|GetActorLocation) (Transformation|GetActorLocation OtherActor))) 0.0) (* "1.000000, 0,0.500000" _knockbackforce) (* "-1.000000, 0,0.500000" _knockbackforce)) true true)
  (Utilities|FlowControl|DoOnce false :!label _label
    (:Completed
      (Audio|PlaySoundatLocation "/Game/GameJam/Audio/SFX/TurkeyNoise_Cue.TurkeyNoise_Cue" (Transformation|GetActorLocation) "0, 0, 0" 0.9 1.0 0.0 0 0 0)
      (Utilities|FlowControl|Delay 0.5)
      (goto _label Reset))))

(event EventBeginPlay
  (bind _returnvalue (Transformation|GetActorLocation))
  (if (Variables|Default|GetFindNearestSurface)
    (bind (_outhit _returnvalue_2) (Collision|SphereTraceByChannel _returnvalue (- _returnvalue "0, 0,2000.000000") 25.0 "TraceTypeQuery1" false 0 "ForOneFrame"))
    (if _returnvalue_2
      (Transformation|SetActorLocation (+ (.Location (Collision|BreakHitResult _outhit)) "0, 0,110.000000") false false)
      (else
        (Development|PrintString (Utilities|String|Append (Utilities|GetObjectName self) " does not have a valid walking surface") true true "(R=0.000000,G=0.897666,B=1.000000,A=1.000000)" 5.0)))))

(event Collision|EventActorBeginOverlap
  (params (OtherActor :type Actor%20Object%20Reference)))

(event EventTick
  (params (DeltaSeconds :type Float%20%28single-precision%29))
  (bind _returnvalue (Transformation|GetActorTransform))
  (bind _returnvalue_2 (Math|Transform|TransformLocation _returnvalue "100.000000, 0, 0"))
  (Utilities|FlowControl|Gate true
    (:Exit
      (bind _outhit (Collision|SphereTraceByChannel _returnvalue_2 (- _returnvalue_2 "0, 0,500.000000") 25.0 "TraceTypeQuery1" false (Utilities|Array|MakeArray (Game|GetPlayerCharacter 0)) "None"))
      (if (or (not (.bBlockingHit (Collision|BreakHitResult _outhit))) (> (.Distance (Collision|BreakHitResult _outhit)) 175.0))
        (Transformation|SetActorRotation (Math|Rotator|Delta(Rotator) (Transformation|GetActorRotation) "0,180.000000, 0"))
        (else
          (Transformation|AddActorLocalOffset (Math|Vector|MakeVector (* (Variables|Default|GetSpeed) DeltaSeconds) 0.0 0.0) false false))))))

(fn ConstructionScript
  (Components|Sphere|SetSphereRadius (Variables|Default|GetActivationSphere) (Variables|Default|GetMovementActivationRange) true))